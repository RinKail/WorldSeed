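; Large layout template for a procedural room-and-corridor generator.
; GenerateRooms scatters overlap-allowed rooms of random footprint around the grid center.
; GenerateCorridors links each room to random rooms with thick, straight-prioritised corridors, looping up to a fixed limit and breaking when ConnectRoom returns false.
; Finish runs the same loop on unconnected rooms using thinner corridors that may overlap.
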(event `self.GenerateRooms`
  (bind (_returnvalue_x _returnvalue_y) (`KismetMathLibrary.BreakVector` (`self.GetRandomScaleInRange` (7.0 7.0 0.0) (20.0 20.0 0.0))))
  (bind (_returnvalue_x_2 _returnvalue_y_2) (`KismetMathLibrary.BreakVector` (`self.GetPositionInRange` (`self.Position`) (200.0 200.0 0.0))))
  (set `self.Position` (/ (`self.GetGridBounds`) 2))
  (for _ (range 61)
    (`self.AddRoom` (`KismetMathLibrary.MakeVector` _returnvalue_x_2 _returnvalue_y_2 2.0) (`KismetMathLibrary.MakeVector` _returnvalue_x _returnvalue_y 5.0) true)))

(event `self.Run`)

(event `self.GenerateCorridors`
  (params (Rooms :type "Array of RoomData Structure (by ref)"))
  (set `self.RandomList` Rooms)
  (for (_array_element _array_index) Rooms
    (`KismetSystemLibrary.PrintString` null (`KismetStringLibrary.Conv_IntToString` _array_index))
    (set `self.bSuccess` false)
    (set `self.RoomAttempts` 0)
    (for _ (range 51)
      (bind _returnvalue (`self.ConnectRoom` _array_element (`self.FindRandomRoom`) 5 false true))
      (if (not _returnvalue)
        (break)))))

(event `self.Finish`
  (for _array_element (`self.GetRoomList`)
    (if (not (`.bIsConnected` (break `RoomData` _array_element)))
      (for _ (range 51)
        (bind _returnvalue (`self.ConnectRoom` _array_element (`self.FindRandomRoom`) 2 true))
        (if (not _returnvalue)
          (break))))))